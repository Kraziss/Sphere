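; BP_RenderTar is a clickable actor that swaps materials on three static mesh components.
; Clicking each box component flips a boolean G and sets material slot 0 of its paired mesh to one of two materials.
; All three boxes share that single G flag, so each click affects which material the next box applies.
; Debug strings print on clicks, and clicking a mesh itself only prints a message.
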(event `self.ReceiveBeginPlay`)

(event `self.Box1.OnClicked`
  (params (TouchedComponent :type "PrimitiveComponent Object Reference") (ButtonPressed :type "Key Structure"))
  (bind _staticmesh1 (`self.StaticMesh1`))
  (`KismetSystemLibrary.PrintString` "Hello")
  (bind _output_get (set `self.G?` (not (`self.G?`))))
  (`/Engine/EditorBlueprintResources/StandardMacros.IsValid` _staticmesh1
    (:`Is Valid`
      (if _output_get
        (`PrimitiveComponent.SetMaterial` _staticmesh1 0 "/Game/Mat/M_Basic_Floor.M_Basic_Floor")
        (`KismetSystemLibrary.PrintString` "1")
        (else
          (`PrimitiveComponent.SetMaterial` _staticmesh1 0 "/Game/Mat/M_Metal_Gold.M_Metal_Gold")
          (`KismetSystemLibrary.PrintString` "2"))))))

(event `self.Box2.OnClicked`
  (params (TouchedComponent :type "PrimitiveComponent Object Reference") (ButtonPressed :type "Key Structure"))
  (bind _staticmesh2 (`self.StaticMesh2`))
  (`KismetSystemLibrary.PrintString` "Hello")
  (bind _output_get (set `self.G?` (not (`self.G?`))))
  (`/Engine/EditorBlueprintResources/StandardMacros.IsValid` _staticmesh2
    (:`Is Valid`
      (if _output_get
        (`PrimitiveComponent.SetMaterial` _staticmesh2 0 "/Game/Mat/M_Metal_Rust.M_Metal_Rust")
        (`KismetSystemLibrary.PrintString` "3")
        (else
          (`PrimitiveComponent.SetMaterial` _staticmesh2 0 "/Game/Mat/M_Ground_Grass.M_Ground_Grass")
          (`KismetSystemLibrary.PrintString` "4"))))))

(event `self.Box3.OnClicked`
  (params (TouchedComponent :type "PrimitiveComponent Object Reference") (ButtonPressed :type "Key Structure"))
  (bind _staticmesh3 (`self.StaticMesh3`))
  (`KismetSystemLibrary.PrintString` "Hello")
  (bind _output_get (set `self.G?` (not (`self.G?`))))
  (`/Engine/EditorBlueprintResources/StandardMacros.IsValid` _staticmesh3
    (:`Is Valid`
      (if _output_get
        (`PrimitiveComponent.SetMaterial` _staticmesh3 0 "/Game/StarterContent/Materials/M_Wood_Floor_Walnut_Polished.M_Wood_Floor_Walnut_Polished")
        (`KismetSystemLibrary.PrintString` "5")
        (else
          (`PrimitiveComponent.SetMaterial` _staticmesh3 0 "/Game/StarterContent/Materials/M_CobbleStone_Rough.M_CobbleStone_Rough")
          (`KismetSystemLibrary.PrintString` "6"))))))

(event `self.StaticMesh1.OnClicked`
  (params (TouchedComponent :type "PrimitiveComponent Object Reference") (ButtonPressed :type "Key Structure"))
  (`KismetSystemLibrary.PrintString` "No"))

(event `self.StaticMesh2.OnClicked`
  (params (TouchedComponent :type "PrimitiveComponent Object Reference") (ButtonPressed :type "Key Structure"))
  (`KismetSystemLibrary.PrintString` "Noo"))

(event `self.StaticMesh3.OnClicked`
  (params (TouchedComponent :type "PrimitiveComponent Object Reference") (ButtonPressed :type "Key Structure"))
  (`KismetSystemLibrary.PrintString` "Noooo"))

(fn `UserConstructionScript`)